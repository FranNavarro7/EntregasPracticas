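; BP_Llave is a key pickup that stays hidden and non-collidable until all its linked key fragments are collected.
; On BeginPlay it counts the FragmentoDeLlave array and binds each fragment's collect event to Collected_Event.
; Once the collected count matches the total, it shows its Sphere and enables Capsule query and physics collision.
; Interactuar sets TieneLlave on the interacting actor and destroys the key.
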(event `self.ReceiveBeginPlay`
  (bind _fragmentodellave (`self.FragmentoDeLlave`))
  (`SceneComponent.SetVisibility` (`self.Sphere`) false false)
  (`PrimitiveComponent.SetCollisionEnabled` (`self.Capsule`) "NoCollision")
  (set `self.FragmentosARecoger` (`KismetArrayLibrary.Array_Length` _fragmentodellave))
  (for _array_element _fragmentodellave
    (add `/Game/TP_N1/BP_ItemFragmentoLlave.AlRecolectar` _array_element (delegate `Collected_Event`))))

(event `Collected_Event`
  (bind _result (`/Engine/EditorBlueprintResources/StandardMacros.IncrementInt` (`self.FragmentosActualesRecogidos`))
    (:`  `
      (if (== _result (`self.FragmentosARecoger`))
        (`SceneComponent.SetVisibility` (`self.Sphere`) true false)
        (`PrimitiveComponent.SetCollisionEnabled` (`self.Capsule`) "QueryAndPhysics")))))

(event `/Game/TP_N1/BPI_Interactuar.Interactuar`
  (params (OtroActor :type "/Game/ThirdPerson/Blueprints/BP_ThirdPersonCharacter Object Reference"))
  (set `/Game/ThirdPerson/Blueprints/BP_ThirdPersonCharacter.TieneLlave` true OtroActor)
  (`self.K2_DestroyActor`))

(fn `UserConstructionScript`)